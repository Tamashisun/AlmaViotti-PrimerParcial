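; BP_Enemigo is an enemy that moves steadily and shoots arrows at a target character.
; A looping timer fires while PuedeDisparar is set, spawning BP_Arrow with velocity along the normalized direction to TargetPersonaje, scaled by VelocidadFlecha.
; Tick offsets it locally by PosicionPersonaje times MultVeloc, without sweep or delta time.
; Setters configure target, movement and firing, though SetVelocidadFlecha writes VeeocidadFlecha rather than the VelocidadFlecha used when firing.
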(event Custom|Disparar
  (if (Variables|Default|GetPuedeDisparar)
    (CallFunction|DisparaFlechaEnemigo (Math|Vector|Normalize (- (Transformation|GetActorLocation (Variables|Default|GetTargetPersonaje)) (Transformation|GetActorLocation))))))

(event EventBeginPlay
  (Utilities|Time|SetTimerbyEvent (delegate Custom|Disparar) (Variables|Default|GetTiempo%20de%20disparo) true false 0.1))

(event EventTick
  (params (DeltaSeconds :type Float%20%28single-precision%29))
  (Transformation|AddActorLocalOffset (* (Variables|Default|GetPosicionPersonaje) (Variables|Default|GetMultVeloc)) false false))

(fn ConstructionScript)

(fn SetPosicionPersonaje
  (params (PosicionPersonaje :type Vector))
  (Variables|Default|SetPosicionPersonaje PosicionPersonaje))

(fn DisparaFlechaEnemigo
  (params (VelovidadNormalizada :type Vector))
  (Game|SpawnActorfromClass "/Game/Arquero_En_Movimiento/BP_Arrow.BP_Arrow_C" (Math|Transform|MakeTransform (Transformation|GetActorLocation) "0, 0, 0" "1.000000,1.000000,1.000000") "Undefined" "MultiplyWithRoot" 0 (* VelovidadNormalizada (Variables|Default|GetVelocidadFlecha)) 0))

(fn SePuedeDisparar
  (params (PuedeDisparar :type Boolean))
  (Variables|Default|SetPuedeDisparar PuedeDisparar))

(fn SetTarget
  (params (TargetPersonaje :type Actor%20Object%20Reference))
  (Variables|Default|SetTargetPersonaje TargetPersonaje))

(fn SetVelocidadFlecha
  (params (VelocidadFlecha :type Vector))
  (Variables|Default|SetVeeocidadFlecha VelocidadFlecha))

(fn SetVelocidadEnemigo
  (params (Velocidad :type Float%20%28double-precision%29))
  (Variables|Default|SetMultVeloc Velocidad))